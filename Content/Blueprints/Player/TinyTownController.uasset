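; Player controller for TinyTown that acts as game coordinator, tracking Book, Food and Gold resources and deciding game end.
; On BeginPlay, after delays, it creates the HUD and spawns turn, event, grid and music managers.
; Selected answers, and starting resources via the same path, update clamped totals, distribute resources per faction on the grid, then end the turn.
; Round end checks extinction, overpopulation, then victory, broadcasting any result.
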(event `self.ReceiveBeginPlay`
  (bind _returnvalue (`self.GetTransform` (`self.K2_GetPawn`)))
  (`KismetSystemLibrary.Delay` 1.0) ; init delay
  (`KismetSystemLibrary.Delay` (`self.animDelayTime`)) ; animation delay
  ;[0 0.5 0] create all necessary game actors and set up refs
  (bind _returnvalue_2 (`|CreateWidget` "/Game/Blueprints/UI/HUD_W.HUD_W_C" null self))
  (bind _output_get (set `self.HUDRef` _returnvalue_2))
  (`UserWidget.AddToViewport` _output_get 0)
  (bind _returnvalue_3 (`|SpawnActorFromClass` "/Game/Blueprints/Turn/TurnController.TurnController_C" _returnvalue "Undefined" "OverrideRootScale" null null))
  (set `self.turnControllerRef` _returnvalue_3)
  (bind _returnvalue_4 (`|SpawnActorFromClass` "/Game/Blueprints/Event/EventController.EventController_C" _returnvalue "Undefined" "OverrideRootScale" null null))
  (bind _output_get_2 (set `self.eventControllerRef` _returnvalue_4))
  (bind _output_get_3 (set `/Game/Blueprints/UI/Event/EventList_W.eventControllerRef` _output_get_2 (`/Game/Blueprints/UI/HUD_W.EventList_W` (`self.HUDRef`))))
  (add `/Game/Blueprints/Event/EventController.onSelectAnswer` _output_get_3 (`|CreateDelegate` :!event `handleSelectAnswer`))
  (bind _returnvalue_5 (`|SpawnActorFromClass` "/Game/Blueprints/Grid/GridManager.GridManager_C" _returnvalue "Undefined" "OverrideRootScale" null null))
  (set `self.GridManagerRef` _returnvalue_5)
  (bind _returnvalue_6 (`|SpawnActorFromClass` "/Game/Blueprints/Music/MusicManager.MusicManager_C" _returnvalue "Undefined" "OverrideRootScale" null null))
  (set `self.musicManagerRef` _returnvalue_6))

(event `startGame`
  (params (delay :type "Float (double-precision)"))
  (`KismetSystemLibrary.Delay` delay)
  (set `self.bShowMouseCursor` true)
  (`WidgetBlueprintLibrary.SetInputMode_GameAndUIEx` self (`self.HUDRef`) "DoNotLock" false)
  (`self.onGameStart`)
  ;[0.5 0.5 0] TODO: REFACTOR: Replace HandleAnswer with AddResource
  (`self.handleSelectAnswer` (make `/Game/Data/Struct/Event/AnswerStruct` "" "" (`self.startResources`))))

(event `handleSelectAnswer`
  (params (AnswerInfo :type "/Game/Data/Struct/Event/AnswerStruct Structure"))
  (bind (_answertext _answerdescription _answerresult) (break `/Game/Data/Struct/Event/AnswerStruct` AnswerInfo))
  (bind _gridmanagerref (`self.GridManagerRef`))
  (bind (_book _food _gold) (break `/Game/Data/Struct/Event/ResourceStruct` _answerresult))
  (`self.addResources` _answerresult)
  ;[0.5 0.5 0] TODO: replace with queue
  (`|ExecutionSequence`
    (:`then_0`
      (`/Game/Blueprints/Grid/GridManager.distributeResource` _gridmanagerref "NewEnumerator1" _book))
    (:`then_1`
      (`/Game/Blueprints/Grid/GridManager.distributeResource` _gridmanagerref "NewEnumerator0" _food))
    (:`then_2`
      (`/Game/Blueprints/Grid/GridManager.distributeResource` _gridmanagerref "NewEnumerator2" _gold)
      (`/Game/Blueprints/Turn/TurnController.endTurn` (`self.turnControllerRef`)))))

(event `onRoundEnd`
  ;[1 1 1] TODO
  (bind (_endgametype _fraction) (`self.checkEndGameCondition`))
  (if (`|EnumInequality` _endgametype "NewEnumerator4")
    (`self.onGameEnd` (make `/Game/Data/Struct/Game/EndGameStruct` _endgametype _fraction (`/Game/Blueprints/Turn/TurnController.dayCount` (`self.turnControllerRef`))))))

(fn `addResources`
  (params (newResoureces :type "/Game/Data/Struct/Event/ResourceStruct Structure (by ref)"))
  (bind (_book _food _gold) (break `/Game/Data/Struct/Event/ResourceStruct` newResoureces))
  (bind (_book_2 _food_2 _gold_2) (break `/Game/Data/Struct/Event/ResourceStruct` (`self.resourcesInfo`)))
  (set `self.resourcesInfo` (make `/Game/Data/Struct/Event/ResourceStruct` (`KismetMathLibrary.Max` (+ _book _book_2)) (`KismetMathLibrary.Max` (+ _food _food_2)) (`KismetMathLibrary.Max` (+ _gold _gold_2)))))

(fn `checkEndGameCondition`
  (returns (EndGameType :type "/Game/Data/Enum/EndGame_E Enum") (Fraction :type "/Game/Data/Enum/Fraction_E Enum"))
  (bind (_isextinction _fraction) (`self.checkExtinction`))
  (bind (_isoverpopulation _fraction_2) (`self.checkOverpopulation`))
  (if _isextinction
    (return "NewEnumerator0" _fraction)
    (elif _isoverpopulation
      (return "NewEnumerator1" _fraction_2)
      (elif (`self.checkWinCondition`)
        (return "NewEnumerator3" "NewEnumerator3")
        (else
          (return "NewEnumerator4" "NewEnumerator3"))))))

(fn `checkExtinction`
  (returns (isExtinction :type Boolean) (fraction :type "/Game/Data/Enum/Fraction_E Enum"))
  (bind (_book _food _gold) (break `/Game/Data/Struct/Event/ResourceStruct` (`self.resourcesInfo`)))
  (if (<= _book 0)
    (return true "NewEnumerator1")
    (elif (<= _food 0)
      (return true "NewEnumerator0")
      (elif (<= _gold 0)
        (return true "NewEnumerator2")
        (else
          (return false "NewEnumerator3"))))))

(fn `checkOverpopulation`
  (returns (isOverpopulation :type Boolean) (fraction :type "/Game/Data/Enum/Fraction_E Enum"))
  (bind _resourcestooverpopulation (`self.resourcesToOverpopulation`))
  (bind (_book _food _gold) (break `/Game/Data/Struct/Event/ResourceStruct` (`self.resourcesInfo`)))
  (if (>= _book _resourcestooverpopulation)
    (return true "NewEnumerator1")
    (elif (>= _food _resourcestooverpopulation)
      (return true "NewEnumerator0")
      (elif (>= _gold _resourcestooverpopulation)
        (return true "NewEnumerator2")
        (else
          (return false "NewEnumerator3"))))))

(fn `checkWinCondition`
  (returns (isWin :type Boolean))
  (bind _resourcestowin (`self.resourcesToWin`))
  (bind (_book _food _gold) (break `/Game/Data/Struct/Event/ResourceStruct` (`self.resourcesInfo`)))
  (return (and (>= _book _resourcestowin) (>= _food _resourcestowin) (>= _gold _resourcestowin))))

(fn `UserConstructionScript`)