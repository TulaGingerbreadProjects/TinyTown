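; Event controller that creates new events in the HUD's event list on turn end and animates the player's answer choice.
; Binds to the turn controller and game instance, whose animation speed sets the timeline's play rate.
; On selection, a timeline lerps a vector packing the clicked button, spacer and other button fill sizes.
; After a delay it broadcasts the chosen answer; it also relays animation skips.
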(event `self.ReceiveBeginPlay`
  (`KismetSystemLibrary.Delay` 0.2)
  (`|ExecutionSequence`
    (:`then_0`
      (bind _astiny_town_controller (cast `/Game/Blueprints/Player/TinyTownController` (`GameplayStatics.GetPlayerController` 0)))
      (set `self.eventListRef` (`/Game/Blueprints/UI/HUD_W.EventList_W` (`/Game/Blueprints/Player/TinyTownController.HUDRef` _astiny_town_controller)))
      (add `/Game/Blueprints/Turn/TurnController.onTurnFinished` (`/Game/Blueprints/Player/TinyTownController.turnControllerRef` _astiny_town_controller) (`|CreateDelegate` :!event `HandeTurnEnd`)))
    (:`then_1`
      (bind _astiny_town_game_instance (cast `/Game/Blueprints/Game/TinyTownGameInstance` (`GameplayStatics.GetGameInstance`)))
      (add `/Game/Blueprints/Game/TinyTownGameInstance.onAnimationSpeedChande` _astiny_town_game_instance (`|CreateDelegate` :!event `updateAnimSpeed`)))))

(event `HandeTurnEnd`
  (params (isRoundEnded :type Boolean))
  (`/Game/Blueprints/UI/Event/EventList_W.createNewEvent` (`self.eventListRef`) isRoundEnded))

(event `updateAnimSpeed`
  (params (newSpeed :type "Float (double-precision)"))
  (bind _output_get (set `self.animSpeed` newSpeed))
  (`TimelineComponent.SetPlayRate` (`self.onClickedButtonTimeline`) _output_get))

(event `handleSelectAnswer`
  (params (eventWidget :type "/Game/Blueprints/UI/Event/Event_W Object Reference") (selectedAnswer :type "/Game/Data/Enum/Direction_E Enum" :default "NewEnumerator0") (AnswerInfo :type "/Game/Data/Struct/Event/AnswerStruct Structure"))
  (bind _size_value (break `SlateChildSize` (`HorizontalBoxSlot.Size` (`self.otherButton`))))
  (bind _size_value_2 (break `SlateChildSize` (`HorizontalBoxSlot.Size` (`self.clickedButton`))))
  (bind _size_value_3 (break `SlateChildSize` (`HorizontalBoxSlot.Size` (`self.spacer`))))
  (bind _output_get (set `self.eventRef` eventWidget))
  (set `self.spacer` (`WidgetLayoutLibrary.SlotAsHorizontalBoxSlot` (`/Game/Blueprints/UI/Event/Event_W.ButtonsSpacer` _output_get)))
  (bind _leftbutton (`/Game/Blueprints/UI/Event/Event_W.LeftButton` _output_get))
  (bind _rightbutton (`/Game/Blueprints/UI/Event/Event_W.RightButton` _output_get))
  (set `self.clickedButton` (`WidgetLayoutLibrary.SlotAsHorizontalBoxSlot` (select `/Game/Data/Enum/Direction_E` selectedAnswer :`NewEnumerator0` _leftbutton :`NewEnumerator1` _rightbutton)))
  (set `self.otherButton` (`WidgetLayoutLibrary.SlotAsHorizontalBoxSlot` (select `/Game/Data/Enum/Direction_E` selectedAnswer :`NewEnumerator0` _rightbutton :`NewEnumerator1` _leftbutton)))
  (set `self.sizeVector` (`KismetMathLibrary.MakeVector` _size_value_2 _size_value_3 _size_value))
  (bind (_direction _alpha) (`Timeline|onClickedButtonTimeline` :!via `PlayFromStart`)
    (:`Update`
      (`HorizontalBoxSlot.SetSize` (`self.clickedButton`) (make `SlateChildSize` (.x (`KismetMathLibrary.VLerp` (`self.sizeVector`) (`self.finalSizeVector`) _alpha))))
      (`HorizontalBoxSlot.SetSize` (`self.spacer`) (make `SlateChildSize` (.y (`KismetMathLibrary.VLerp` (`self.sizeVector`) (`self.finalSizeVector`) _alpha))))
      (`HorizontalBoxSlot.SetSize` (`self.otherButton`) (make `SlateChildSize` (.z (`KismetMathLibrary.VLerp` (`self.sizeVector`) (`self.finalSizeVector`) _alpha)))))
    (:`Finished`
      (`KismetSystemLibrary.Delay` (`self.delayAfterEventAnimation`))
      (`self.onSelectAnswer` AnswerInfo))))

(event `skipAnimation`
  (`self.onSkipAnimation`))

(fn `UserConstructionScript`)