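; BeatenHeart is an environment actor that pulses its scale continuously to simulate a beating heart.
; On BeginPlay it stores its current scale and derives a beaten scale that is smaller by a fixed amount on each axis.
; A timeline lerps the actor between the two scales, then after a short delay the Beat event calls itself to repeat the pulse indefinitely.
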(event `self.ReceiveBeginPlay`
  (bind _output_get (set `self.normalScale` (`self.GetActorScale3D`)))
  (set `self.beatenScale` (- _output_get (0.2 0.2 0.2)))
  (`self.beat`))

(event `beat`
  (bind (_direction _alpha) (`Timeline|beatTimeline` :!via `PlayFromStart`)
    (:`Update`
      (`self.SetActorScale3D` (`KismetMathLibrary.VLerp` (`self.normalScale`) (`self.beatenScale`) _alpha)))
    (:`Finished`
      (`KismetSystemLibrary.Delay` 0.1)
      (`self.beat`))))

(fn `UserConstructionScript`)