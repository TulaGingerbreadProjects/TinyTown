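; Turn controller that advances a four-phase day cycle, animating the time-of-day lighting whenever a turn ends.
; A timeline rotates the directional light toward the next phase's angle, updating the sky sphere and recapturing the skylight each tick.
; On finish it broadcasts turn completion, and each full cycle increments the day count and notifies the player controller of round end.
; Bound events let the animation be skipped or sped up.
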(event `self.ReceiveBeginPlay`
  (`KismetSystemLibrary.Delay` 0.2)
  ;[1 1 1] Set all light refs
  (bind _outactors (`GameplayStatics.GetAllActorsOfClass` "/Script/Engine.DirectionalLight"))
  (set `self.LightSourceRef` (`|GetArrayItem` _outactors))
  (bind _outactors_2 (`GameplayStatics.GetAllActorsOfClass` "/Script/Engine.SkyLight"))
  (set `self.skyLightRef` (`|GetArrayItem` _outactors_2))
  (bind _outactors_3 (`GameplayStatics.GetAllActorsOfClass` "/Engine/EngineSky/BP_Sky_Sphere.BP_Sky_Sphere_C"))
  (set `self.skySphereRef` (`|GetArrayItem` _outactors_3))
  (set `self.endRotation` (`self.K2_GetActorRotation` (`self.LightSourceRef`)))
  (`TimelineComponent.SetPlayRate` (`self.switchTurnTimeline`) (`self.switchTurnMultiplier`))
  (`|ExecutionSequence`
    (:`then_0`
      (bind _astiny_town_controller (cast `/Game/Blueprints/Player/TinyTownController` (`GameplayStatics.GetPlayerController` 0)))
      (bind _output_get (set `self.eventControllerRef` (`/Game/Blueprints/Player/TinyTownController.eventControllerRef` _astiny_town_controller)))
      (add `/Game/Blueprints/Event/EventController.onSkipAnimation` _output_get (`|CreateDelegate` :!event `handleSkipAnimation`)))
    (:`then_1`
      (bind _astiny_town_game_instance (cast `/Game/Blueprints/Game/TinyTownGameInstance` (`GameplayStatics.GetGameInstance`)))
      (add `/Game/Blueprints/Game/TinyTownGameInstance.onAnimationSpeedChange` _astiny_town_game_instance (`|CreateDelegate` :!event `updateAnimSpeed`)))))

(event `updateAnimSpeed`
  (params (newSpeed :type "Float (double-precision)"))
  (bind _output_get (set `self.animSpeed` newSpeed))
  (`TimelineComponent.SetPlayRate` (`self.switchTurnTimeline`) (* _output_get (`self.switchTurnMultiplier`))))

(event `handleSkipAnimation`
  (bind _switchturntimeline (`self.switchTurnTimeline`))
  (`TimelineComponent.SetNewTime` _switchturntimeline (`TimelineComponent.GetTimelineLength` _switchturntimeline)))

(event `endTurn`
  (set `self.startRotation` (`self.endRotation`))
  (set `self.endRotation` (`BlueprintMapLibrary.Map_Find` (`self.angles`) (`self.turnPhaze`)))
  (bind (_direction _alpha) (`Timeline|switchTurnTimeline` :!via `PlayFromStart`)
    (:`Update`
      (`self.K2_SetActorRotation` (`self.LightSourceRef`) (`KismetMathLibrary.RLerp` (`self.startRotation`) (`self.endRotation`) _alpha true) false)
      (`SkyLightComponent.RecaptureSky` (`SkyLight.LightComponent` (`self.skyLightRef`)))
      (`/Engine/EngineSky/BP_Sky_Sphere.UpdateSunDirection` (`self.skySphereRef`)))
    (:`Finished`
      (bind _output_get (set `self.turnPhaze` (mod (+ (`self.turnPhaze`) 1) 4)))
      (if (== _output_get 0)
        (`/Engine/EditorBlueprintResources/StandardMacros.IncrementInt` (`self.dayCount`)
          (:`  `
            (bind _astiny_town_controller (cast `/Game/Blueprints/Player/TinyTownController` (`GameplayStatics.GetPlayerController` 0)))
            (`/Game/Blueprints/Player/TinyTownController.onRoundEnd` _astiny_town_controller)
            (`self.onTurnFinished` true)))
        (else
          (`self.onTurnFinished` false))))))

(fn `UserConstructionScript`)