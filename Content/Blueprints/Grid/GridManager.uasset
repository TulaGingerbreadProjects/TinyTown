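; Grid manager for TinyTown that spawns a square grid of tiles and spreads resource gains and losses across them by fraction.
; After a short startup delay it spawns tiles with staggered delays, then tells TinyTownController to start the game.
; DistributeResource recursively passes leftovers on, filling an unfinished house or random empty tile for gains and draining the lowest-count house for losses.
; Grid expansion and AddNewResourcesToGrid are TODO stubs.
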(event `self.ReceiveBeginPlay`
  ;[1 1 1] Spawn grid and Start game
  (`KismetSystemLibrary.Delay` 2.0)
  (bind _astiny_town_controller (cast `/Game/Blueprints/Player/TinyTownController` (`GameplayStatics.GetPlayerController` 0)))
  (set `self.controllerRef` _astiny_town_controller)
  (`self.spawnGrid`))

(event `onGridSpawned`
  (params (spawnDelay :type "Float (double-precision)"))
  ;[1 1 1] Spawn grid and Start game
  (`/Game/Blueprints/Player/TinyTownController.startGame` (`self.controllerRef`) (+ spawnDelay (`self.delayAfterGridSpawned`))))

(fn `AddNewResourcesToGrid`
  (params (newResources :type "/Game/Data/Struct/Event/ResourceStruct Structure"))
  ;[1 1 1] TODO: queue
)

(fn `distributeResource`
  (params (fraction :type "/Game/Data/Enum/Fraction_E Enum" :default "NewEnumerator3") (resource :type Integer))
  (locals (local_fraction :type "/Game/Data/Enum/Fraction_E Enum" :default "NewEnumerator3") (local_resources :type Integer))
  (bind _local_fraction (`local.local_fraction`))
  (bind _local_fraction_2 (`local.local_fraction`))
  (set `local.local_fraction` fraction)
  (bind _output_get (set `local.local_resources` resource))
  (`/Engine/EditorBlueprintResources/StandardMacros.CompareInt` _output_get
    (:`>`
      (bind _result (`self.findTileToAdd` _local_fraction))
      (`/Engine/EditorBlueprintResources/StandardMacros.IsValid` _result
        (:`Is Valid`
          (bind _reminder (`/Game/Blueprints/Grid/gridTile.addResources` _result _local_fraction (`local.local_resources`)))
          (`self.distributeResource` (`local.local_fraction`) _reminder))))
    (:`<`
      (bind _result_2 (`self.findTileToReduce` _local_fraction_2))
      (`/Engine/EditorBlueprintResources/StandardMacros.IsValid` _result_2
        (:`Is Valid`
          (bind _reminder_2 (`/Game/Blueprints/Grid/gridTile.addResources` _result_2 _local_fraction_2 (`local.local_resources`)))
          (`self.distributeResource` (`local.local_fraction`) _reminder_2))))))

(fn `expandGrid`
  (params (numberOfNewRows :type Integer))
  ;[0.5 0.5 0] TODO: expand grid
)

(fn `findTileToAdd`
  (params (fraction :type "/Game/Data/Enum/Fraction_E Enum" :default "NewEnumerator3"))
  (returns (result :type "/Game/Blueprints/Grid/gridTile Object Reference"))
  (locals (local_fraction :type "/Game/Data/Enum/Fraction_E Enum" :default "NewEnumerator3") (local_results :type "Array of /Game/Blueprints/Grid/gridTile Object Reference") (local_findFractionHouse :type Boolean))
  (bind _local_results (`local.local_results`))
  (bind _local_results_2 (`local.local_results`))
  (set `local.local_fraction` fraction)
  (for _array_element (`self.tilesRef`)
    (for _array_element_2 (break `/Game/Data/Struct/Grid/RowStruct` _array_element)
      (if (`|EnumEquality` (`/Game/Blueprints/Grid/gridTile.fraction` _array_element_2) (`local.local_fraction`))
        ;[0 0.5 0] leave only 1 elem in array, because we have no more then 1 not finished house at a time
        (if (< (`/Game/Blueprints/Grid/gridTile.count` _array_element_2) 3)
          (set `local.local_findFractionHouse` true)
          (`KismetArrayLibrary.Array_Clear` _local_results_2)
          (`KismetArrayLibrary.Array_Add` _local_results_2 _array_element_2))
        (else
          ;[0 0.5 0] add all NONE tiles to randomize position of new house
          (if (and (not (`local.local_findFractionHouse`)) (`|EnumEquality` (`/Game/Blueprints/Grid/gridTile.fraction` _array_element_2) "NewEnumerator3"))
            (`KismetArrayLibrary.Array_Add` (`local.local_results`) _array_element_2))))))
  (return (`|GetArrayItem` _local_results (`KismetMathLibrary.RandomInteger` (`KismetArrayLibrary.Array_Length` _local_results)))))

(fn `findTileToReduce`
  (params (fraction :type "/Game/Data/Enum/Fraction_E Enum" :default "NewEnumerator3"))
  (returns (result :type "/Game/Blueprints/Grid/gridTile Object Reference"))
  (locals (local_result :type "/Game/Blueprints/Grid/gridTile Object Reference") (local_fraction :type "/Game/Data/Enum/Fraction_E Enum" :default "NewEnumerator3") (local_min :type Integer :default 4))
  (set `local.local_fraction` fraction)
  (for _array_element (`self.tilesRef`)
    (for _array_element_2 (break `/Game/Data/Struct/Grid/RowStruct` _array_element)
      (if (`|EnumEquality` (`/Game/Blueprints/Grid/gridTile.fraction` _array_element_2) (`local.local_fraction`))
        ;[1 1 1] Find house with min resources
        (if (< (`/Game/Blueprints/Grid/gridTile.count` _array_element_2) (`local.local_min`))
          (set `local.local_min` (`/Game/Blueprints/Grid/gridTile.count` _array_element_2))
          (set `local.local_result` _array_element_2)))))
  (return (`local.local_result`)))

(fn `spawnGrid`
  (locals (local_rowIndex :type Integer) (local_columnIndex :type Integer) (local_gridOffset :type Integer :default 0))
  (bind _gridrotation (`self.GridRotation`))
  (bind _output_tiles (break `/Game/Data/Struct/Grid/RowStruct` (`|GetArrayItem` (`self.tilesRef`) (`local.local_rowIndex`))))
  (bind _returnvalue (* (+ (* (`local.local_rowIndex`) (`self.gridSize`)) (`local.local_columnIndex`)) (`self.delayBetweenGrids`)))
  (set `local.local_gridOffset` (/ (`self.gridSize`) 2))
  (for _index (range (`self.gridSize`))
    (set `local.local_rowIndex` _index)
    (`KismetArrayLibrary.Array_Add` (`self.tilesRef`)) ; Add empty row to fill it with tiles
    (for _index_2 (range (`self.gridSize`))
      (set `local.local_columnIndex` _index_2)
      (bind _returnvalue_2 (`|SpawnActorFromClass` "/Game/Blueprints/Grid/gridTile.gridTile_C" (`KismetMathLibrary.MakeTransform` (+ (`self.K2_GetActorLocation`) (`KismetMathLibrary.GreaterGreater_VectorRotator` (`KismetMathLibrary.MakeVector` (* (- (`local.local_rowIndex`) (`local.local_gridOffset`)) (.x (`self.tileSize`))) (* (- (`local.local_columnIndex`) (`local.local_gridOffset`)) (.y (`self.tileSize`))) -500.0) _gridrotation)) _gridrotation) "Undefined" "OverrideRootScale" null _returnvalue (`self.offset`) null))
      (`KismetArrayLibrary.Array_Add` _output_tiles _returnvalue_2)))
  (`self.onGridSpawned` _returnvalue))

(fn `UserConstructionScript`)