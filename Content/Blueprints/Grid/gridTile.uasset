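; Grid tile actor that holds an owning Fraction and a resource Count from zero to three.
; AddResources sets the Fraction, clamps the new count and returns the overflow, while UpdateTile resets the Fraction on empty tiles and refreshes a debug text label.
; At BeginPlay, a delayed timeline lerps the tile by an offset before updating it.
; A looping timer is set up to rotate the debug label toward the camera.
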(event `updateTile`
  ;[0.5 0.5 0] TODO: Mesh animation
  (if (== (`self.count`) 0)
    (set `self.fraction` "NewEnumerator3"))
  ;;[0.5 0 0.5] DEBUG: Update FractionText
  (`TextRenderComponent.K2_SetText` (`self.FractionText`) (`|FormatText` "{Fraction} {Count}" (`KismetTextLibrary.Conv_StringToText` (`|GetEnumeratorNameAsString` (`self.fraction`))) (`self.count`))))

(event `self.ReceiveBeginPlay`
  (`self.updateLocation`)
  ;[0.5 0 0.5] DEBUG: Rotate FractionText
  (`KismetSystemLibrary.K2_SetTimerDelegate` (`|CreateDelegate` :!event `updateRotation`) 1.0 true))

(event `updateRotation`
  ;[0.5 0 0.5] DEBUG: Rotate FractionText
  (`SceneComponent.K2_SetWorldRotation` (`self.FractionText`) (`KismetMathLibrary.FindLookAtRotation` (`self.K2_GetActorLocation`) (`PlayerCameraManager.GetCameraLocation` (`PlayerController.PlayerCameraManager` (`GameplayStatics.GetPlayerController` 0)))) false false))

(event `updateLocation`
  ;[0 0.5 0] Update actor location when game start
  (bind _output_get (set `self.startLocation` (`self.K2_GetActorLocation`)))
  (set `self.endLocation` (+ _output_get (`self.offset`)))
  (`KismetSystemLibrary.Delay` (`self.delayTime`))
  (bind (_direction _alpha) (`Timeline|liftTimeLine` :!via `PlayFromStart`)
    (:`Update`
      (`self.K2_SetActorLocation` (`KismetMathLibrary.VLerp` (`self.startLocation`) (`self.endLocation`) _alpha)))
    (:`Finished`
      (`self.updateTile`))))

(fn `addResources`
  (params (Fraction :type "/Game/Data/Enum/Fraction_E Enum" :default "NewEnumerator3") (resources :type Integer))
  (returns (reminder :type Integer))
  (locals (local_sum :type Integer :default 0))
  (set `self.fraction` Fraction)
  (bind _output_get (set `local.local_sum` (+ resources (`self.count`))))
  (set `self.count` (`KismetMathLibrary.Clamp` _output_get 0 3))
  (`self.updateTile`)
  (return (`KismetMathLibrary.Clamp` (- (`local.local_sum`) (`self.count`)) -3 3)))

(fn `UserConstructionScript`
  (`self.updateTile`))