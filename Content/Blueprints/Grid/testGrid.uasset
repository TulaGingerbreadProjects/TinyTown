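; testGrid is a grid actor Blueprint that lines itself up with the level's player start and sizes a preview of the grid.
; Its construction script calls the parent script, then moves the actor to the first PlayerStart found.
; When ShouldSpawnGrid is set, it scales the GridPreview component by GridSize with a flattened Z axis; no grid cells are spawned here.
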(fn `UserConstructionScript`
  (`parent.UserConstructionScript`)
  (bind _outactors (`GameplayStatics.GetAllActorsOfClass` "/Script/Engine.PlayerStart"))
  (`self.K2_SetActorLocation` (`self.K2_GetActorLocation` (`|GetArrayItem` _outactors)))
  (if (`self.shouldSpawnGrid`)
    (`SceneComponent.SetWorldScale3D` (`self.gridPreview`) (* (1.0 1.0 0.1) (`self.gridSize`)))))